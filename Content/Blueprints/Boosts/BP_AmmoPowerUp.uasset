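; BP_AmmoPowerUp is a boost that gives the activating player extra ammo.
; On activation it stores the player, casts it to ShooterCharacter and adds one magazine's worth of ammo to the current weapon's CurrentAmmo, with no clamp applied here.
; On expiry it only defers to the parent handler, as both branches of its validity check on the stored player are empty.
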(event `self.OnActivated`
  (params (ActivateFor :type "Actor Object Reference"))
  (set `self.ActivatedForPlayer` ActivateFor)
  (bind _asshooter_character (cast `ShooterCharacter` ActivateFor))
  (bind _currentweapon (`ShooterCharacter.CurrentWeapon` _asshooter_character))
  (set `BaseWeapon.CurrentAmmo` (+ (`BaseWeapon.CurrentAmmo` _currentweapon) (`BaseWeapon.MagazineSize` _currentweapon)) _currentweapon))

(event `self.OnExpired`
  (`/Engine/EditorBlueprintResources/StandardMacros.IsValid` (`self.ActivatedForPlayer`)
    (:`Is Valid`
      _)
    (:`Is Not Valid`
      _))
  (`parent.OnExpired`))

(fn `UserConstructionScript`
  (`parent.UserConstructionScript`))