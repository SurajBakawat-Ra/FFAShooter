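; Shooter character Blueprint that sets up the player's on-screen HUD and keeps its health display current.
; On BeginPlay it creates the player HUD and a helmet-mounted display, hiding the latter's shield bar and putting the health bar on top.
; It binds to the health component's change event to update the bar fill as a fraction of default health.
; The helmet display is removed when health reaches zero.
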(event `self.ReceiveBeginPlay`
  (`|ExecutionSequence`
    (:`then_0`
      (bind _returnvalue (`|CreateWidget` "/Game/UI/WBP_PlayerHUD.WBP_PlayerHUD_C"))
      (`UserWidget.AddToViewport` _returnvalue 0))
    (:`then_1`
      (bind _returnvalue_2 (`|CreateWidget` "/Game/UI/PlayerHUD/Widget_HelmetMountedDisplay.Widget_HelmetMountedDisplay_C"))
      (set `self.HealthWidget` _returnvalue_2)
      (`UserWidget.AddToViewport` _returnvalue_2 0)
      (`/Game/UI/PlayerHUD/Widget_HelmetMountedDisplay.SetShieldBarVisibility` (`self.HealthWidget`) "Hidden")
      (`/Game/UI/PlayerHUD/Widget_HelmetMountedDisplay.SetHealthBarOnTop` (`self.HealthWidget`))
      (add `HealthComponent.OnHealthChanged` (`self.HealthComp`) (delegate `OnHealthChanged_Event`)))))

(event `OnHealthChanged_Event`
  (params (HealthComp :type "HealthComponent Object Reference") (Health :type "Float (single-precision)") (HealthDelta :type "Float (single-precision)") (DamageType :type "DamageType Object Reference") (InstigatedBy :type "Controller Object Reference") (DamageCauser :type "Actor Object Reference"))
  (bind _healthwidget (`self.HealthWidget`))
  (`/Game/UI/HealthBar/Widget_HealthBar.UpdateHealthBarFill` (`/Game/UI/PlayerHUD/Widget_HelmetMountedDisplay.GetHealthBar` _healthwidget) (/ Health (`HealthComponent.DefaultHealth` (`self.HealthComp`))))
  (if (<= Health 0.0)
    (`Widget.RemoveFromParent` _healthwidget)))

(fn `UserConstructionScript`)